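; Gameplay HUD Blueprint that shows the owning player's ping as a debug on-screen message.
; Each tick, once the owning PlayerController and its PlayerState are valid, it prints the ping in milliseconds through PrintString.
; The print key depends on whether the controller has authority, so authority and non-authority readouts each replace their own line.
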(event EventBeginPlay)

(event Collision|EventActorBeginOverlap
  (params (OtherActor :type Actor%20Object%20Reference)))

(event EventTick
  (params (DeltaSeconds :type Float%20%28single-precision%29))
  (bind _returnvalue (Game|Player|GetOwningPlayerController))
  (bind _playerstate (Variables|/Script/Engine.Controller|GetPlayerState _returnvalue))
  (Utilities|IsValid _returnvalue
    (:Is%20Valid
      (Utilities|IsValid _playerstate
        (:Is%20Valid
          (Development|PrintString (Utilities|String|Append "Ping:" (Utilities|String|ToString(Float) (Class|PlayerState|GetPinginMilliseconds _playerstate))) true true "(R=0.000000,G=0.660000,B=1.000000,A=1.000000)" 2.0 (Utilities|String|StringToName (Utilities|String|ToString(Integer) (Math|Integer|SelectInt 0 1 (Ability|HasAuthority _returnvalue))))))))))

(fn ConstructionScript)