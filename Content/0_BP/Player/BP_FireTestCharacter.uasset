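; BP_FireTestCharacter is a player character that starts with a test rifle equipped, apparently for testing weapon fire.
; On BeginPlay it links the base weapon anim layer to the mesh, then after a short delay gets the inventory from its PRPlayerState.
; It requests the DA_TestRifle item, waits again, and equips the inventory's first weapon through WeaponManagerComponent, relying on fixed delays for sequencing.
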(event EventBeginPlay
  (Components|SkeletalMesh|AnimationBlueprintLinking|LinkAnimClassLayers (Variables|Character|GetMesh) "/Game/2_Characters/RCharacter/Animation/AnimLayers/ABP_WeaponAnimLayerBase.ABP_WeaponAnimLayerBase_C")
  (Utilities|FlowControl|Delay 0.2)
  (bind _asplayer_controller (Utilities|Casting|CastToPlayerController (Pawn|GetController)))
  (bind _asprplayer_state (Utilities|Casting|CastToPRPlayerState (Variables|/Script/Engine.Controller|GetPlayerState _asplayer_controller)))
  (Variables|Default|SetIventory (Class|PRPlayerState|GetInventoryComponent _asprplayer_state))
  (Class|PRInventoryComponent|RequestAddWeaponItem (Class|PRPlayerState|GetInventoryComponent _asprplayer_state) "/Game/0_BP/EquipmentSystem/Data/DA_TestRifle.DA_TestRifle")
  (Utilities|FlowControl|Delay 0.2)
  (Class|PRWeaponManagerComponent|EquipWeapon (Variables|Default|GetWeaponManagerComponent) (Class|PRInventoryComponent|GetWeaponItematIndex (Variables|Default|GetIventory))))

(fn ConstructionScript)