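; BP_PlayerCharacter is the player character Blueprint, holding BPTest functions that exercise the inventory.
; Each function casts PlayerState to PRPlayerState and sends a request to its inventory component.
; The requests add a given weapon, add the fixed test heal mod, or equip a mod to a weapon.
; The equip function uses its indices crosswise: WeaponIndex selects the mod and ModIndex selects the weapon.
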(fn ConstructionScript)

(fn BPTestAddWeaponItem
  (params (WeaponData :type PR%20Weapon%20Data%20Asset%20Object%20Reference))
  (bind _asprplayer_state (Utilities|Casting|CastToPRPlayerState (Variables|Default|GetPlayerState)))
  (Class|PRInventoryComponent|RequestAddWeaponItem (Class|PRPlayerState|GetInventoryComponent _asprplayer_state) WeaponData))

(fn BPTestAddModItem
  (bind _asprplayer_state (Utilities|Casting|CastToPRPlayerState (Variables|Default|GetPlayerState)))
  (Class|PRInventoryComponent|RequestAddModItem (Class|PRPlayerState|GetInventoryComponent _asprplayer_state) "/Game/0_BP/Data/Mod/DA_TestMod_Heal.DA_TestMod_Heal"))

(fn BPTestEquipModtoWeapon
  (params (ModIndex :type Integer) (WeaponIndex :type Integer))
  (bind _asprplayer_state (Utilities|Casting|CastToPRPlayerState (Variables|Default|GetPlayerState)))
  (Class|PRInventoryComponent|RequestEquipModItemtoWeapon (Class|PRPlayerState|GetInventoryComponent _asprplayer_state) (Class|PRInventoryComponent|GetModItematIndex (Class|PRPlayerState|GetInventoryComponent _asprplayer_state) WeaponIndex) (Class|PRInventoryComponent|GetWeaponItematIndex (Class|PRPlayerState|GetInventoryComponent _asprplayer_state) ModIndex)))