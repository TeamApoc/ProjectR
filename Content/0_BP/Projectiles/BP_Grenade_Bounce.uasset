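; Bouncing grenade projectile that lives up to five seconds and deals an area effect when destroyed.
; On destruction it spawns a Niagara explosion, then, with projectile authority, sphere-traces around itself while ignoring its instigator.
; Visibility line traces filter out targets behind walls, and each remaining unique actor receives the effect once through ApplyEffectToTargetWithHit.
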(event EventBeginPlay
  (Actor|SetLifeSpan 5.0))

(event Collision|EventActorBeginOverlap
  (params (OtherActor :type Actor%20Object%20Reference)))

(event EventTick
  (params (DeltaSeconds :type Float%20%28single-precision%29)))

(event EventOnProjectileDestroyed
  (Niagara|SpawnSystematLocation "/Game/3_Effects/Explosion/FX/NS_Basic_Explosion_01.NS_Basic_Explosion_01" (Transformation|GetActorLocation) "0, 0, 0" "1.000000,1.000000,1.000000" true true "AutoRelease")
  (if (Class|PRProjectileBase|HasProjectileAuthority)
    (Utilities|Set|Clear (Variables|Default|GetHitActors))
    (bind _outhits (Collision|MultiSphereTraceByChannel (Transformation|GetActorLocation) "0, 0, 0" (Variables|Default|GetRadius) "TraceTypeQuery3" false (Utilities|Array|MakeArray (Game|GetInstigator)) "None"))
    (bind _array_element (Utilities|Array|ForEachLoopwithBreak _outhits)
      (:LoopBody
        ;[0.15 0.15 0.15 0.5] 벽 차폐 확인
        (bind _returnvalue (Collision|LineTraceByChannel (Transformation|GetActorLocation) (Transformation|GetActorLocation (.HitActor (Collision|BreakHitResult _array_element))) "TraceTypeQuery1" false (Utilities|Array|MakeArray (.HitActor (Collision|BreakHitResult _array_element))) "None"))
        (if (not _returnvalue)
          (Utilities|IsValid (.HitActor (Collision|BreakHitResult _array_element))
            (:Is%20Valid
              (if (not (Utilities|Set|Contains (Variables|Default|GetHitActors) (.HitActor (Collision|BreakHitResult _array_element))))
                (Utilities|Set|Add (Variables|Default|GetHitActors) (.HitActor (Collision|BreakHitResult _array_element)))
                (Class|PRProjectileBase|ApplyEffecttoTargetwithHit (.HitActor (Collision|BreakHitResult _array_element)) _array_element)))))))))

(fn ConstructionScript)