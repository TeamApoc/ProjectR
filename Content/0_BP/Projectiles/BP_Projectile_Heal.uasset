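; Healing projectile that bursts into a ring-of-heal effect with sound when destroyed.
; Overlapping a player character destroys it, except the owner's own character while the projectile should bounce.
; On destruction, the projectile authority sphere-traces the radius and applies the configured effect once to each unique actor hit.
; It has a fixed lifespan and still contains debug prints and a debug sphere.
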(event OnComponentBeginOverlap(DetectPawnCollsion)
  (params (OverlappedComponent :type Primitive%20Component%20Object%20Reference) (OtherActor :type Actor%20Object%20Reference) (OtherComp :type Primitive%20Component%20Object%20Reference) (OtherBodyIndex :type Integer) (bFromSweep :type Boolean) (SweepResult :type Hit%20Result%20Structure%20%28by%20ref%29))
  (bind _returnvalue (Components|GetOwner))
  (bind _asprplayer_character (Utilities|Casting|CastToPRPlayerCharacter OtherActor))
  (Utilities|IsValid _asprplayer_character
    (:Is%20Valid
      (Development|PrintString (Utilities|GetDisplayName _returnvalue))
      (if (== (Pawn|GetController _asprplayer_character) _returnvalue)
        (if (Class|PRProjectileBase|GetShouldBounce)
          (Development|PrintString "true")
          (else
            (Development|PrintString "false")
            (Class|PRProjectileBase|DestroyProjectile "Impact" :!label _label)))
        (else
          (goto _label))))))

(event EventBeginPlay
  (Actor|SetLifeSpan 2e+01))

(event EventOnProjectileDestroyed
  (bind _returnvalue (Transformation|GetActorLocation))
  (Niagara|SpawnSystematLocation "/Game/Assets/MegaMagicVFXBundle/VFX/MagicAuraVFX/VFX/RingOfFlames/Systems/N_RingOfHeal.N_RingOfHeal" _returnvalue "0, 0, 0" "1.000000,1.000000,1.000000" true true "AutoRelease")
  (Audio|PlaySoundatLocation "/Game/Assets/Weapon/Meridian/Sound/Explode/SC_Meridian_Projectile_Explode.SC_Meridian_Projectile_Explode" _returnvalue "0, 0, 0" 1.0 1.0 0.0 0 0 0 0)
  (Rendering|Debug|DrawDebugSphere (Transformation|GetActorLocation) (Variables|Default|GetRadius) 12 "(R=1.000000,G=0.070387,B=0.000000,A=1.000000)" 1.0)
  (if (Class|PRProjectileBase|HasProjectileAuthority)
    (Utilities|Set|Clear (Variables|Default|GetHitActors))
    (bind _outhits (Collision|MultiSphereTraceByChannel (Transformation|GetActorLocation) "0, 0, 0" (Variables|Default|GetRadius) "TraceTypeQuery3" false 0 "None"))
    (bind _array_element (Utilities|Array|ForEachLoopwithBreak _outhits)
      (:LoopBody
        (Variables|Default|SetArray%20Element _array_element)
        (bind _output_get (Variables|Default|SetHit%20Actor (.HitActor (Collision|BreakHitResult _array_element))))
        (Utilities|IsValid _output_get
          (:Is%20Valid
            (if (not (Utilities|Set|Contains (Variables|Default|GetHitActors) (Variables|Default|GetHit%20Actor)))
              (Utilities|Set|Add (Variables|Default|GetHitActors) (Variables|Default|GetHit%20Actor))
              (Class|PRProjectileBase|ApplyEffecttoTargetwithHit (Variables|Default|GetHit%20Actor) (Variables|Default|GetArray%20Element)))))))))

(fn ConstructionScript)