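; BP_PickableMod is a test pickup actor that labels itself with the name of the item it offers.
; It scans its InteractableComponent's interaction actions for PRInteraction_TestPickUpItem entries with valid ItemData and writes the display name into its W_WorldText widget.
; The same logic is duplicated in the Construction Script and BeginPlay, so the label is set both at construction and when play begins.
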(event EventBeginPlay
  (bind _asw_world_text (Utilities|Casting|CastToW_WorldText (UserInterface|GetWidget (Variables|Default|GetWidget))))
  (for _array_element (Variables|/Script/ProjectR.PRInteractableComponent|GetInteractionActions (Variables|Default|GetInteractableComponent))
    (bind _asprinteraction_test_pick_up_item (Utilities|Casting|CastToPRInteraction_TestPickUpItem _array_element))
    (Utilities|IsValid (Variables|/Script/ProjectR.PRInteraction_TestPickUpItem|GetItemData _asprinteraction_test_pick_up_item)
      (:Is%20Valid
        (Default|SetText _asw_world_text (Class|PRItemDataAsset|GetDisplayName (Variables|/Script/ProjectR.PRInteraction_TestPickUpItem|GetItemData _asprinteraction_test_pick_up_item)))))))

(event Collision|EventActorBeginOverlap
  (params (OtherActor :type Actor%20Object%20Reference)))

(event EventTick
  (params (DeltaSeconds :type Float%20%28single-precision%29)))

(fn ConstructionScript
  (bind _asw_world_text (Utilities|Casting|CastToW_WorldText (UserInterface|GetWidget (Variables|Default|GetWidget))))
  (for _array_element (Variables|/Script/ProjectR.PRInteractableComponent|GetInteractionActions (Variables|Default|GetInteractableComponent))
    (bind _asprinteraction_test_pick_up_item (Utilities|Casting|CastToPRInteraction_TestPickUpItem _array_element))
    (Utilities|IsValid (Variables|/Script/ProjectR.PRInteraction_TestPickUpItem|GetItemData _asprinteraction_test_pick_up_item)
      (:Is%20Valid
        (Default|SetText _asw_world_text (Class|PRItemDataAsset|GetDisplayName (Variables|/Script/ProjectR.PRInteraction_TestPickUpItem|GetItemData _asprinteraction_test_pick_up_item)))))))