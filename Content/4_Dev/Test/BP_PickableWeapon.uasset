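; BP_PickableWeapon is a weapon pickup actor that displays its assigned WeaponData through a colored visual and a world-space name label.
; The construction script applies ColorTarget to the Niagara effect, point light and cylinder's custom primitive data, then sets the label and calls RefreshVisual.
; BeginPlay sets the label again, using the WeaponData object name or an "Invalid Weapon" fallback.
; No pickup logic appears in these graphs.
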(event EventBeginPlay
  (bind _weapondata (Variables|Default|GetWeaponData))
  (bind _asw_world_text (Utilities|Casting|CastToW_WorldText (UserInterface|GetWidget (Variables|Default|GetWidget))))
  (Utilities|IsValid _weapondata
    (:Is%20Valid
      (Default|SetText _asw_world_text (Utilities|Text|ToText(String) (Utilities|GetObjectName _weapondata))))
    (:Is%20Not%20Valid
      (Default|SetText _asw_world_text "Invalid Weapon"))))

(fn ConstructionScript
  (bind _weapondata (Variables|Default|GetWeaponData))
  (bind _color_target (Variables|Default|GetColor%20Target))
  (bind _cylinder1 (Variables|Default|GetCylinder1))
  (bind (_r _g _b _a) (Math|Color|BreakColor _color_target))
  (Utilities|FlowControl|Sequence
    (:then_0
      (Niagara|SetNiagaraVariable(LinearColor) (Variables|Default|GetNS_JumpDemo) "Color" _color_target)
      (Rendering|Components|Light|SetLightColor (Variables|Default|GetPointLight) _color_target true)
      (Rendering|Material|SetDefaultCustomPrimitiveDataFloat _cylinder1 0 1.0)
      (Rendering|Material|SetDefaultCustomPrimitiveDataVector4 _cylinder1 1 (Math|Vector4|MakeVector4 _r _g _b _a)))
    (:then_1
      (bind _asw_world_text (Utilities|Casting|CastToW_WorldText (UserInterface|GetWidget (Variables|Default|GetWidget))))
      (Utilities|IsValid _weapondata
        (:Is%20Valid
          (Default|SetText _asw_world_text (Utilities|Text|ToText(String) (Utilities|GetObjectName _weapondata))))
        (:Is%20Not%20Valid
          (Default|SetText _asw_world_text "Invalid Weapon"))))
    (:then_2
      (Class|PRPickableWeapon|RefreshVisual))))