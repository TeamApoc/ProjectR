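; Test player character that drives the inventory and weapon equipment system through hard-coded debug keys.
; Keys request test rifle, pistol and mod items from the PRPlayerState inventory component, and attach a mod to a weapon there.
; Other keys call WeaponManagerComponent to equip inventory weapons, unequip or switch Primary/Secondary slots, and toggle armed state.
; The mod-equip helper uses its ModIndex and WeaponIndex swapped, harmless only because both are passed as zero.
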(event Input|KeyboardEvents|6
  (params (Key :type Key%20Structure :default "None"))
  (:Pressed
    (CallFunction|BPTestEquipModtoWeapon)))

(event Input|KeyboardEvents|5
  (params (Key :type Key%20Structure :default "None"))
  (:Pressed
    (CallFunction|BPTestAddModItem)))

(event Input|KeyboardEvents|2
  (params (Key :type Key%20Structure :default "None"))
  ;[0.15 0.15 0.15 0.5] 무기 슬롯 전환
  (:Pressed
    (Class|PRWeaponManagerComponent|SetCurrentWeaponSlot (Variables|Default|GetWeaponManagerComponent) "Secondary")))

(event Input|KeyboardEvents|Z
  (params (Key :type Key%20Structure :default "None"))
  ;[0.15 0.15 0.15 0.5] 무기 장착 - 인벤톡리 아이템
  (:Pressed
    (Class|PRWeaponManagerComponent|EquipInventoryWeaponatIndex (Variables|Default|GetWeaponManagerComponent))))

(event Input|KeyboardEvents|1
  (params (Key :type Key%20Structure :default "None"))
  ;[0.15 0.15 0.15 0.5] 무기 슬롯 전환
  (:Pressed
    (Class|PRWeaponManagerComponent|SetCurrentWeaponSlot (Variables|Default|GetWeaponManagerComponent) "Primary")))

(event Input|KeyboardEvents|4
  (params (Key :type Key%20Structure :default "None"))
  ;[0.15 0.15 0.15 0.5] 아이템 추가
  (:Pressed
    (CallFunction|BPTestAddWeaponItem "/Game/0_BP/Data/Weapon/DA_Pistol.DA_Pistol")))

(event Input|KeyboardEvents|X
  (params (Key :type Key%20Structure :default "None"))
  ;[0.15 0.15 0.15 0.5] 무기 장착 - 인벤톡리 아이템
  (:Pressed
    (Class|PRWeaponManagerComponent|EquipInventoryWeaponatIndex (Variables|Default|GetWeaponManagerComponent) 1)))

(event Input|KeyboardEvents|3
  (params (Key :type Key%20Structure :default "None"))
  ;[0.15 0.15 0.15 0.5] 아이템 추가
  (:Pressed
    (CallFunction|BPTestAddWeaponItem "/Game/0_BP/Data/Weapon/DA_AssaultRifle.DA_AssaultRifle")))

(event Input|KeyboardEvents|F
  (params (Key :type Key%20Structure :default "None"))
  ;[0.15 0.15 0.15 0.5] 무장/비무장 전환
  (:Pressed
    (switch Utilities|FlowControl|Switch|SwitchonEPRArmedState (Class|PRWeaponManagerComponent|GetArmedState (Variables|Default|GetWeaponManagerComponent))
      (:Armed
        (Class|PRWeaponManagerComponent|SetWeaponArmedState (Variables|Default|GetWeaponManagerComponent) "Unarmed"))
      (:Unarmed
        (Class|PRWeaponManagerComponent|SetWeaponArmedState (Variables|Default|GetWeaponManagerComponent) "Armed")))))

(event Input|KeyboardEvents|C
  (params (Key :type Key%20Structure :default "None"))
  ;[0.15 0.15 0.15 0.5] 무기 해제
  (:Pressed
    (Class|PRWeaponManagerComponent|UnequipWeaponfromSlot (Variables|Default|GetWeaponManagerComponent) "Primary")))

(event Input|KeyboardEvents|V
  (params (Key :type Key%20Structure :default "None"))
  ;[0.15 0.15 0.15 0.5] 무기 해제
  (:Pressed
    (Class|PRWeaponManagerComponent|UnequipWeaponfromSlot (Variables|Default|GetWeaponManagerComponent) "Secondary")))

(fn ConstructionScript)

(fn BPTestAddWeaponItem
  (params (WeaponData :type PR%20Weapon%20Data%20Asset%20Object%20Reference))
  (bind _asprplayer_state (Utilities|Casting|CastToPRPlayerState (Variables|Default|GetPlayerState)))
  (Class|PRInventoryComponent|RequestAddWeaponItem (Class|PRPlayerState|GetInventoryComponent _asprplayer_state) WeaponData))

(fn BPTestAddModItem
  (bind _asprplayer_state (Utilities|Casting|CastToPRPlayerState (Variables|Default|GetPlayerState)))
  (Class|PRInventoryComponent|RequestAddModItem (Class|PRPlayerState|GetInventoryComponent _asprplayer_state) "/Game/0_BP/Data/Mod/DA_TestMod.DA_TestMod"))

(fn BPTestEquipModtoWeapon
  (params (ModIndex :type Integer) (WeaponIndex :type Integer))
  (bind _asprplayer_state (Utilities|Casting|CastToPRPlayerState (Variables|Default|GetPlayerState)))
  (Class|PRInventoryComponent|RequestEquipModItemtoWeapon (Class|PRPlayerState|GetInventoryComponent _asprplayer_state) (Class|PRInventoryComponent|GetModItematIndex (Class|PRPlayerState|GetInventoryComponent _asprplayer_state) WeaponIndex) (Class|PRInventoryComponent|GetWeaponItematIndex (Class|PRPlayerState|GetInventoryComponent _asprplayer_state) ModIndex)))